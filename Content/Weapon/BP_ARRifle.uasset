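; BP_ARRifle is an AR rifle pickup that the player collects by touching it.
; A Timeline, told to Play on every Tick, drives the yaw of StaticMesh1 to rotate the rifle.
; When an FPSPlayer overlaps the Capsule and its CheckWeapon is false, the pickup prints a debug message, calls EquipWeaponMessage on that player and destroys itself.
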(event OnComponentBeginOverlap(Capsule)
  (params (OverlappedComponent :type Primitive%20Component%20Object%20Reference) (OtherActor :type Actor%20Object%20Reference) (OtherComp :type Primitive%20Component%20Object%20Reference) (OtherBodyIndex :type Integer) (bFromSweep :type Boolean) (SweepResult :type Hit%20Result%20Structure%20%28by%20ref%29))
  (bind _asfpsplayer (Utilities|Casting|CastToFPSPlayer OtherActor))
  (if (not (Variables|/Script/FPSRPG.FPSPlayer|GetCheckWeapon _asfpsplayer))
    (Development|PrintText "equip")
    (Class|BPCharacterInterFace|EquipWeapon(Message) _asfpsplayer)
    (Actor|DestroyActor)))

(event EventBeginPlay)

(event Collision|EventActorBeginOverlap
  (params (OtherActor :type Actor%20Object%20Reference)))

(event EventTick
  (params (DeltaSeconds :type Float%20%28single-precision%29))
  (bind _rotator (Timeline|타임라인_0 Play)
    (:Update
      (Transformation|SetRelativeRotation (Variables|Default|GetStaticMesh1) (Math|Rotator|MakeRotator 0.0 0.0 _rotator) false false))))

(fn ConstructionScript)