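; BP_Jet is a jet that flies straight along its facing direction once its StartFly event is called.
; StartFly toggles the static mesh's visibility on every call, but starts the jet sound and sets the Start flag only the first time.
; While Start is set, Tick feeds the actor's forward vector into CharacterMovement as input, with no stop logic.
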(event Collision|EventActorBeginOverlap
  (params (OtherActor :type Actor%20Object%20Reference)))

(event EventTick
  (params (DeltaSeconds :type Float%20%28single-precision%29))
  (if (Variables|Default|Getstart)
    (Class|PawnMovementComponent|AddInputVector (Variables|Character|GetCharacterMovement) (Math|Vector|GetForwardVector (Transformation|GetActorRotation)) false)))

(event EventStartFly
  (Rendering|ToggleVisibility (Variables|Default|GetStaticMesh) false)
  (if (not (Variables|Default|Getstart))
    (Audio|Components|Audio|SetSound (Variables|Default|GetAudio) "/Game/Sound/jetfly_Cue.jetfly_Cue")
    (Audio|Components|Audio|Play (Variables|Default|GetAudio) 0.0)
    (Variables|Default|Setstart true)))

(fn ConstructionScript)