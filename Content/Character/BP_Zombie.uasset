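; BP_Zombie is a melee enemy character that chases the player and attacks at close range.
; A Tick-driven state machine moves between Idle, Follow and Attack by player distance, steering with direct movement input rather than pathfinding.
; Attack start/end events toggle a hit capsule that deals randomized damage to FPSPlayer, while an animation-end event repeats or abandons the attack.
; Point damage reduces HP, with headshots killing instantly; death plays a montage and disables collision.
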(event OnComponentBeginOverlap(Capsule)
  (params (OverlappedComponent :type Primitive%20Component%20Object%20Reference) (OtherActor :type Actor%20Object%20Reference) (OtherComp :type Primitive%20Component%20Object%20Reference) (OtherBodyIndex :type Integer) (bFromSweep :type Boolean) (SweepResult :type Hit%20Result%20Structure%20%28by%20ref%29))
  (bind _atk (Variables|Default|GetAtk))
  ;[1 1 1] Apply Damage
  (if (not (== OtherActor self))
    (if (not (== OtherActor "BP_Zombie"))
      (bind _asfpsplayer (Utilities|Casting|CastToFPSPlayer OtherActor))
      (Game|Damage|ApplyDamage _asfpsplayer (Math|Random|RandomFloatinRange _atk (+ _atk 2e+01)) 0 self))))

(event Custom|SaveDisAndDir
  (bind _returnvalue (Game|GetPlayerCharacter 0))
  (bind _returnvalue_2 (Transformation|GetActorLocation))
  (bind _returnvalue_3 (Transformation|GetActorLocation _returnvalue))
  (bind _returnvalue_4 (- _returnvalue_3 _returnvalue_2))
  (Variables|Default|SetDistancePlayer (Math|Vector|VectorLength _returnvalue_4))
  (Variables|Default|SetDirToPlayer (Math|Vector|Normalize _returnvalue_4)))

(event Custom|OnAnimEndAttack
  (Variables|Default|SetIsAttacking false)
  (if (>= (Variables|Default|GetDistancePlayer) 1.8e+02)
    (Variables|Default|SetCurrentState "NewEnumerator1")
    (else
      (Animation|PlayAnimMontage "/Game/zombie/Zombie_Attack_mixamo_com_Montage.Zombie_Attack_mixamo_com_Montage" 1.0 "None")
      (Variables|Default|SetIsAttacking true))))

(event Custom|Custom%20Event_0
  (Audio|PlaySound2D "/Game/zombie/189281__huminaatio__zombie-breathing.189281__huminaatio__zombie-breathing"))

(event Custom|OnCallEndAttack
  (Collision|SetCollisionEnabled (Variables|Default|GetCapsule) "NoCollision"))

(event Custom|OnCallStartAttack
  (Collision|SetCollisionEnabled (Variables|Default|GetCapsule) "QueryAndPhysics"))

(event Game|Damage|EventPointDamage
  (params (Damage :type Float%20%28single-precision%29) (DamageType :type Damage%20Type%20Object%20Reference) (HitLocation :type Vector :default "0, 0, 0") (HitNormal :type Vector :default "0, 0, 0") (HitComponent :type Primitive%20Component%20Object%20Reference) (BoneName :type Name :default "None") (ShotFromDirection :type Vector :default "0, 0, 0") (InstigatedBy :type Controller%20Object%20Reference) (DamageCauser :type Actor%20Object%20Reference) (HitInfo :type Hit%20Result%20Structure%20%28by%20ref%29))
  (if (Utilities|Name|Equal(Name) BoneName "Head")
    (Variables|Default|SetHP 0.0)
    (Development|PrintString "HeadShot!")
    (Variables|Default|Setis%20death true :!label _label)
    (Animation|PlayAnimMontage "/Game/zombie/Zombie_Dying_mixamo_com_Montage.Zombie_Dying_mixamo_com_Montage" 1.0 "None")
    (Collision|SetCollisionEnabled (Variables|Character|GetMesh) "NoCollision")
    (Collision|SetCollisionEnabled (Variables|Collision|GetCapsuleComponent) "NoCollision")
    (else
      (bind _output_get (Variables|Default|SetHP (- (Variables|Default|GetHP) Damage)))
      (Development|PrintString (Utilities|String|ToString(Float) _output_get))
      (if (<= (Variables|Default|GetHP) 0.0)
        (goto _label)))))

(event EventTick
  (params (DeltaSeconds :type Float%20%28single-precision%29))
  (if (not (Variables|Default|Getis%20death))
    (CallFunction|SaveDisandDir)
    (switch Utilities|FlowControl|Switch|SwitchonZombieState (Variables|Default|GetCurrentState)
      (:NewEnumerator0
        (if (<= (Variables|Default|GetDistancePlayer) 1.2e+03)
          (Variables|Default|SetCurrentState "NewEnumerator1")))
      (:NewEnumerator1
        (if (<= (Variables|Default|GetDistancePlayer) 8e+01)
          (Variables|Default|SetCurrentState "NewEnumerator2")
          (Animation|PlayAnimMontage "/Game/zombie/Zombie_Attack_mixamo_com_Montage.Zombie_Attack_mixamo_com_Montage" 1.0 "None")
          (Variables|Default|SetIsAttacking true)
          (else
            (Pawn|Input|AddMovementInput (Variables|Default|GetDirToPlayer) 1.0 false))))
      (:NewEnumerator2
        (if (not (Variables|Default|GetIsAttacking))
          (if (>= (Variables|Default|GetDistancePlayer) 9e+01)
            (Variables|Default|SetCurrentState "NewEnumerator1")))))))

(fn ConstructionScript)