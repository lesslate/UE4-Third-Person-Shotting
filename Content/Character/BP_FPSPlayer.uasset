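; BP_FPSPlayer is the player character that picks up, swaps and aims an AR4 rifle and a crossbow.
; The Interaction input collects tagged weapons by sphere overlap, while prompt events set a widget component's text.
; Keys 1 and 2 swap hand and back meshes with a montage once both weapons are owned.
; Aiming switches rotation mode, shows a crosshair and drives camera FOV through a timeline.
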(event EventBeginPlay
  (bind _returnvalue (Game|GetPlayerController 0))
  (bind _returnvalue_2 (UserInterface|CreateWidget "/Game/UI/BP_Crosshair.BP_Crosshair_C" _returnvalue))
  (Variables|Default|SetCrossHair _returnvalue_2)
  (bind _returnvalue_3 (UserInterface|CreateWidget "/Game/UI/BP_Widget.BP_Widget_C" _returnvalue))
  (UserInterface|Viewport|AddtoViewport _returnvalue_3 0)
  (Widget|SetVisibility _returnvalue_3 "Visible")
  (Rendering|SetVisibility (Variables|Default|GetWidget_Interaction) false false))

(event Collision|EventActorBeginOverlap
  (params (OtherActor :type Actor%20Object%20Reference)))

(event EventTick
  (params (DeltaSeconds :type Float%20%28single-precision%29)))

(event EventGetBolt
  (Variables|Default|SetRemainBolt (+ (Variables|Default|GetRemainBolt) 5)))

(event EventGetAmmo
  (Variables|Default|SetRemainAmmo (+ (Variables|Default|GetRemainAmmo) 30)))

(event EventWeaponText
  (bind _aswidget_bp_interaction (Utilities|Casting|CastToWidgetBP_Interaction (UserInterface|GetUserWidgetObject (Variables|Default|GetWidget_Interaction))))
  (Variables|/Game/UI/WidgetBP_Interaction.WidgetBP_Interaction_C|SetInteractionText _aswidget_bp_interaction "AR4")
  (Rendering|SetVisibility (Variables|Default|GetWidget_Interaction) true true))

(event EventWeaponTextEnd
  (Rendering|SetVisibility (Variables|Default|GetWidget_Interaction) false false))

(event EventCrossBowText
  (bind _aswidget_bp_interaction (Utilities|Casting|CastToWidgetBP_Interaction (UserInterface|GetUserWidgetObject (Variables|Default|GetWidget_Interaction))))
  (Variables|/Game/UI/WidgetBP_Interaction.WidgetBP_Interaction_C|SetInteractionText _aswidget_bp_interaction "Cross Bow")
  (Rendering|SetVisibility (Variables|Default|GetWidget_Interaction) true true))

(event EventCrossBowTextEnd
  (Rendering|SetVisibility (Variables|Default|GetWidget_Interaction) false false))

(event Input|ActionEvents|InputActionAiming
  (params (Key :type Key%20Structure))
  (bind _checkbow (Variables|Default|GetCheckBow))
  (bind _isreloading (Variables|Default|GetIsReloading))
  (bind _charactermovement (Variables|Character|GetCharacterMovement))
  (bind _checkweapon (Variables|Default|GetCheckWeapon))
  (bind _issprint (Variables|Default|GetIsSprint))
  (bind _charactermovement_2 (Variables|Character|GetCharacterMovement))
  (bind _returnvalue (or _checkbow _checkweapon))
  (:Pressed
    (if (not _isreloading)
      (if _returnvalue
        (if (not _issprint)
          (Variables|/Script/Engine.CharacterMovementComponent|SetbUseControllerDesiredRotation _charactermovement_2 true)
          (Variables|/Script/Engine.CharacterMovementComponent|SetbOrientRotationToMovement _charactermovement_2 false)
          (Variables|Default|SetAiming true)
          (UserInterface|Viewport|AddtoViewport (Variables|Default|GetCrossHair) 0)
          (bind _fov (Timeline|타임라인 Play)
            (:Update
              (Camera|SetFieldOfView (Variables|Default|GetFollowCamera) _fov)))))))
  (:Released
    (if (not _isreloading)
      (if _returnvalue
        (if (not _issprint)
          (Variables|/Script/Engine.CharacterMovementComponent|SetbUseControllerDesiredRotation _charactermovement false)
          (Variables|/Script/Engine.CharacterMovementComponent|SetbOrientRotationToMovement _charactermovement true)
          (Variables|Default|SetAiming false)
          (Widget|RemovefromParent (Variables|Default|GetCrossHair))
          (Timeline|타임라인 Reverse))))))

(event Input|ActionEvents|InputActionInteraction
  (params (Key :type Key%20Structure))
  (:Pressed
    (bind _outactors (Collision|SphereOverlapActors (Transformation|GetActorLocation) 2e+02 (Utilities|Array|MakeArray "ObjectTypeQuery9") 0))
    (for _array_element _outactors
      (if (Actor|ActorHasTag _array_element "AR4")
        (if (not (Variables|Default|GetCheckWeapon))
          (Actor|DestroyActor _array_element)
          (Components|StaticMesh|SetStaticMesh (Variables|Default|GetWeaponMesh) "/Game/FPS_Weapon_Bundle/Weapons/Meshes/AR4/SM_AR4.SM_AR4")
          (Variables|Default|SetCheckWeapon true))
        (elif (Actor|ActorHasTag _array_element "CrossBow")
          (if (not (Variables|Default|GetCheckBow))
            (Actor|DestroyActor _array_element)
            (Components|StaticMesh|SetStaticMesh (Variables|Default|GetSecondWeaponBack) "/Game/Item/crossbow_Mesh_0358.crossbow_Mesh_0358")
            (Variables|Default|SetCheckBow true)))))))

(event Input|KeyboardEvents|1
  (params (Key :type Key%20Structure))
  (:Pressed
    (if (Variables|Default|GetBowState)
      (if (not (or (Variables|Default|GetAiming) (Variables|Default|GetIsReloading)))
        (if (and (Variables|Default|GetCheckWeapon) (Variables|Default|GetCheckBow))
          (Animation|PlayAnimMontage "/Game/Character/Swat/SwatAnim/Standing_Disarm_Over_Shoulder_Montage.Standing_Disarm_Over_Shoulder_Montage" 1.0 "None")
          (Components|StaticMesh|SetStaticMesh (Variables|Default|GetWeaponBack) 0)
          (Components|StaticMesh|SetStaticMesh (Variables|Default|GetSecondWeaponMesh) 0)
          (Components|StaticMesh|SetStaticMesh (Variables|Default|GetWeaponMesh) "/Game/FPS_Weapon_Bundle/Weapons/Meshes/AR4/SM_AR4.SM_AR4")
          (Components|StaticMesh|SetStaticMesh (Variables|Default|GetSecondWeaponBack) "/Game/Item/crossbow_Mesh_0358.crossbow_Mesh_0358")
          (Variables|Default|SetBowState false))))))

(event Input|KeyboardEvents|2
  (params (Key :type Key%20Structure))
  (:Pressed
    (if (not (Variables|Default|GetBowState))
      (if (not (or (Variables|Default|GetAiming) (Variables|Default|GetIsReloading)))
        (if (and (Variables|Default|GetCheckWeapon) (Variables|Default|GetCheckBow))
          (Animation|PlayAnimMontage "/Game/Character/Swat/SwatAnim/Standing_Disarm_Over_Shoulder_Montage.Standing_Disarm_Over_Shoulder_Montage" 1.0 "None")
          (Components|StaticMesh|SetStaticMesh (Variables|Default|GetWeaponBack) "/Game/FPS_Weapon_Bundle/Weapons/Meshes/AR4/SM_AR4.SM_AR4")
          (Components|StaticMesh|SetStaticMesh (Variables|Default|GetSecondWeaponMesh) "/Game/Item/crossbow_Mesh_0358.crossbow_Mesh_0358")
          (Components|StaticMesh|SetStaticMesh (Variables|Default|GetWeaponMesh) 0)
          (Components|StaticMesh|SetStaticMesh (Variables|Default|GetSecondWeaponBack) 0)
          (Variables|Default|SetBowState true))))))

(fn ConstructionScript)