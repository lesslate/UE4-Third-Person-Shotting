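; BP_Zombie2 is a zombie Blueprint that shows on-screen damage feedback whenever it takes damage.
; On AnyDamage it creates a headshot or regular damage HUD widget based on the IsHead flag, passes it the damage amount and adds it to the viewport.
; The widget's initial position is the zombie's location projected to screen space with a fixed offset.
; IsHead resets after each headshot display and is not set in these graphs.
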(event EventBeginPlay)

(event Collision|EventActorBeginOverlap
  (params (OtherActor :type Actor%20Object%20Reference)))

(event EventTick
  (params (DeltaSeconds :type Float%20%28single-precision%29)))

(event Game|Damage|EventAnyDamage
  (params (Damage :type Float%20%28single-precision%29) (DamageType :type Damage%20Type%20Object%20Reference) (InstigatedBy :type Controller%20Object%20Reference) (DamageCauser :type Actor%20Object%20Reference))
  (bind _returnvalue (Game|GetPlayerController 0))
  (bind _returnvalue_2 (Transformation|GetActorLocation))
  (bind _screenposition (Class|GameplayStatics|ProjectWorldtoScreen _returnvalue _returnvalue_2 false))
  (bind _returnvalue_3 (+ _screenposition "(X=-50.000000,Y=-100.000000)"))
  (if (Variables|Default|GetIsHead)
    (bind _returnvalue_4 (UserInterface|CreateWidget "/Game/UI/BP_HeadDamageHUD.BP_HeadDamageHUD_C" 0 _returnvalue_3 Damage))
    (UserInterface|Viewport|AddtoViewport _returnvalue_4 0)
    (Variables|Default|SetIsHead false)
    (else
      (bind _returnvalue_5 (UserInterface|CreateWidget "/Game/UI/BP_DamageHUD.BP_DamageHUD_C" 0 _returnvalue_3 Damage))
      (UserInterface|Viewport|AddtoViewport _returnvalue_5 0))))

(fn ConstructionScript)