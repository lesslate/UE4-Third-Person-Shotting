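; BP_Bomb is an environment bomb actor that explodes once when its Bomb event is triggered.
; After a random delay of a few seconds, it swaps the particle system to an explosion effect, plays an explosion sound and applies massive, full radial damage over a wide radius.
; An IsBombed flag, set only after the blast, blocks later triggers.
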(event EventBomb
  (if (not (Variables|Default|GetIsBombed))
    (Utilities|FlowControl|Delay (Math|Random|RandomFloatinRange 4.0 6.0))
    (Effects|Components|ParticleSystem|SetTemplate (Variables|Default|GetParticleSystem) "/Game/StarterContent/Particles/P_Explosion.P_Explosion")
    (Audio|Components|Audio|SetSound (Variables|Default|GetAudio) "/Game/Sound/Explosioncue.Explosioncue")
    (Audio|Components|Audio|Play (Variables|Default|GetAudio) 0.0)
    (Game|Damage|ApplyRadialDamage (Math|Random|RandomFloatinRange 2.3e+05 3e+05) (Transformation|GetActorLocation) 3e+03 0 0 self 0 true "ECC_Visibility")
    (Variables|Default|SetIsBombed true)))

(fn ConstructionScript)

(fn NewFunction0)